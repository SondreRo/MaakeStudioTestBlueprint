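; BP_GameModeMain is a game mode that adds a MiniMapHud widget to the viewport on BeginPlay and loads the MuseumDay level on Reset.
; It manages placed cameras through functions that spawn them into the PlacedCams array, delete one, or clear all.
; SpawnPlayerNPC spawns an NPC at NpcStartPos only when GetActorOfClass finds no existing instance of it.
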(event `Reset`
  (`GameplayStatics.OpenLevel` "MuseumDay"))

(event `self.ReceiveBeginPlay`
  (bind _returnvalue (`|CreateWidget` "/Game/Blueprints/MiniMap/MiniMapHud.MiniMapHud_C" (`GameplayStatics.GetPlayerController` 0)))
  (`UserWidget.AddToViewport` _returnvalue 0))

(fn `ClearAllCam`
  (for _array_element (`self.PlacedCams`)
    (`self.K2_DestroyActor` _array_element))
  (`KismetArrayLibrary.Array_Clear` (`self.PlacedCams`)))

(fn `DeleteOneCam`
  (params (CamToDelete :type "Actor Object Reference"))
  (`KismetArrayLibrary.Array_RemoveItem` (`self.PlacedCams`) CamToDelete)
  (`self.K2_DestroyActor` CamToDelete))

(fn `SpawnCam`
  (params (CamToSpawn :type "Actor Class Reference") (CamTransform :type "Transform Structure"))
  (bind _returnvalue (`|SpawnActorFromClass` CamToSpawn CamTransform "Undefined" "OverrideRootScale" null null))
  (`KismetArrayLibrary.Array_Add` (`self.PlacedCams`) _returnvalue))

(fn `SpawnPlayerNPC`
  (bind _actortospawn (`self.ActorToSpawn`))
  (bind _returnvalue (`GameplayStatics.GetActorOfClass` _actortospawn))
  (if (not (`KismetSystemLibrary.IsValid` _returnvalue))
    (`|SpawnActorFromClass` _actortospawn (`KismetMathLibrary.Conv_VectorToTransform` (`self.NpcStartPos`)) "Undefined" "OverrideRootScale" null null)))

(fn `UserConstructionScript`)