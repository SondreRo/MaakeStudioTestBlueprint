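; VaultDoor is a door that opens once both of its two switches have been flipped.
; FlippedSwitch records the switch by index in the Switches array, applies the Flipped material to the matching switch component, then calls CheckDoors.
; When both entries are true, CheckDoors triggers OpenDoor, whose Timeline drives the Cube's relative Z location to animate the opening.
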(event `OpenDoor`
  (bind (_direction _dooropen) (`Timeline|Timeline`)
    (:`Update`
      (`SceneComponent.K2_SetRelativeLocation` (`self.Cube`) (`KismetMathLibrary.MakeVector` 0.0 0.0 _dooropen) false false))))

(fn `CheckDoors`
  (bind _switches (`self.Switches`))
  (if (and (`|GetArrayItem` _switches 1) (`|GetArrayItem` _switches))
    (`self.OpenDoor`)))

(fn `FlippedSwitch`
  (params (SwitchNr :type Integer))
  (if (== SwitchNr 0)
    (`PrimitiveComponent.SetMaterial` (`self.Switch1`) 0 "/Game/Blueprints/GameObjects/Flipped.Flipped"))
  (if (== SwitchNr 1)
    (`PrimitiveComponent.SetMaterial` (`self.Switch2`) 0 "/Game/Blueprints/GameObjects/Flipped.Flipped"))
  (`KismetArrayLibrary.Array_Set` (`self.Switches`) SwitchNr true)
  (`self.CheckDoors`))

(fn `UserConstructionScript`)