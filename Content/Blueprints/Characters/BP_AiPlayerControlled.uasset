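; AI-driven character Blueprint that walks to a preset start position and notifies interactable actors it overlaps.
; After a short delay on BeginPlay, it issues an AI Move To toward NpcStartWalkPos.
; Every Tick, FinishedMoving scans all overlapping actors and sends NPCInteractMessage to those implementing the NPC_Interact interface, regardless of whether the move has finished.
; The MoveTo function and construction script are empty.
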(event `self.ReceiveBeginPlay`
  (`KismetSystemLibrary.Delay` 2.0)
  (`|AIMoveTo` self (`self.NpcStartWalkPos`) null))

(event `self.ReceiveTick`
  (params (DeltaSeconds :type "Float (single-precision)"))
  (`self.FinishedMoving`))

(fn `FinishedMoving`
  (for _array_element (`self.GetOverlappingActors` null)
    (if (`KismetSystemLibrary.DoesImplementInterface` _array_element "/Game/Blueprints/GameObjects/NPC_Interact.NPC_Interact_C")
      (message `/Game/Blueprints/GameObjects/NPC_Interact.NPC_Interact` _array_element))))

(fn `MoveTo`)

(fn `UserConstructionScript`)